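; Prototype musket weapon actor that lets the player fire bullets.
; On BeginPlay it caches the Player character, enables its own input and creates a Prototype_BuildingMusket widget as ReloadHUD, without displaying it here.
; Pressing Shoot while the player is alive, aiming and able to shoot calls TakeAmmo on the Player and spawns a Prototype_Bullet at the Arrow component's transform.
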(event `self.ReceiveBeginPlay`
  (bind _asplayer (cast `/Game/Placeable/Player` (`GameplayStatics.GetPlayerCharacter` 0)))
  (set `self.Player` _asplayer)
  (`self.EnableInput` (`GameplayStatics.GetPlayerController` 0))
  (bind _returnvalue (`|CreateWidget` "/Game/Blueprints/Widgets/Prototype_BuildingMusket.Prototype_BuildingMusket_C"))
  (set `self.ReloadHUD` _returnvalue))

(event `InputAction|Shoot`
  (params (Key :type "Key Structure"))
  (:`Pressed`
    (if (`/Game/Placeable/Player.bIsDead` (`self.Player`))
      _
      (elif (`/Game/Placeable/Player.bIsAiming` (`self.Player`))
        (if (`/Game/Placeable/Player.bCanShoot` (`self.Player`))
          (`/Game/Placeable/Player.TakeAmmo` (`self.Player`))
          (`|SpawnActorFromClass` "/Game/Blueprints/Prototype_Bullet.Prototype_Bullet_C" (`SceneComponent.K2_GetComponentToWorld` (`self.Arrow`)) "AlwaysSpawn" "OverrideRootScale" null null))))))

(fn `UserConstructionScript`)