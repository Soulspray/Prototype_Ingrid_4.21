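; Prototype player controller that handles the inventory screen and quitting the game.
; On BeginPlay it creates the inventory widget, adds it to the viewport and caches the Player character.
; The Inventory input, ignored while the player is dead, flip-flops between opening and closing the widget, unless an animation is playing.
; Each toggle switches cursor visibility and input mode, zeroing look input scales while open and restoring them on close.
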(event `self.ReceiveBeginPlay`
  (bind _returnvalue (`|CreateWidget` "/Game/Blueprints/Widgets/Prototype_Inventory.Prototype_Inventory_C"))
  (bind _output_get (set `self.InventoryRef` _returnvalue))
  (`UserWidget.AddToViewport` _output_get 0)
  (bind _asplayer (cast `/Game/Placeable/Player` (`GameplayStatics.GetPlayerCharacter` 0)))
  (set `self.PlayerRef` _asplayer))

(event `InputAction|Inventory`
  (params (Key :type "Key Structure"))
  (:`Pressed`
    (if (not (`/Game/Placeable/Player.bIsDead` (`self.PlayerRef`)))
      (`self.OpenAndCloseInventory`))))

(event `InputAction|Quit`
  (params (Key :type "Key Structure"))
  (:`Pressed`
    (`KismetSystemLibrary.QuitGame` null "Quit")))

(fn `UserConstructionScript`)