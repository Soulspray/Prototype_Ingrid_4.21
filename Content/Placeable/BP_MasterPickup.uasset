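; Master pickup actor that gives the player ammo or musket parts when they press Interact.
; The construction script looks up the Item enum in a data table for mesh, particle and name, and applies box and mesh transforms.
; Player overlap toggles a name-and-key prompt widget and the actor's input.
; Interacting switches on item type to grant it, then destroys the actor; health-giving logic exists but is unconnected.
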(event `self.ReceiveBeginPlay`
  (bind _returnvalue (`|CreateWidget` "/Game/Blueprints/Widgets/Prototype_Item_Pickup.Prototype_Item_Pickup_C"))
  (set `self.HUD` _returnvalue)
  (bind _asplayer (cast `/Game/Placeable/Player` (`GameplayStatics.GetPlayerCharacter` 0)))
  (set `self.Player` _asplayer)
  (bind _asprototype_controller (cast `/Game/Blueprints/PrototypeController` (`GameplayStatics.GetPlayerController` 0)))
  (set `self.PlayerControllerRef` _asprototype_controller))

(event `InputAction|Interact`
  (params (Key :type "Key Structure"))
  (:`Pressed`
    (`Widget.RemoveFromParent` (`self.HUD`))
    (`self.ItemFunction`)
    (`KismetSystemLibrary.Delay` 0.05)
    (`self.K2_DestroyActor`)))

(event `self.Box.OnComponentBeginOverlap`
  (params (OverlappedComponent :type "PrimitiveComponent Object Reference") (OtherActor :type "Actor Object Reference") (OtherComp :type "PrimitiveComponent Object Reference") (OtherBodyIndex :type Integer) (bFromSweep :type Boolean) (SweepResult :type "HitResult Structure (by ref)"))
  (cast `/Game/Placeable/Player` OtherActor)
  (`self.WidgetWork` :!label _label))

(event `self.Box.OnComponentEndOverlap`
  (params (OverlappedComponent :type "PrimitiveComponent Object Reference") (OtherActor :type "Actor Object Reference") (OtherComp :type "PrimitiveComponent Object Reference") (OtherBodyIndex :type Integer))
  (cast `/Game/Placeable/Player` OtherActor)
  (goto _label :!via `EndOverlap`))

(fn `ItemFunction`
  (switch `/Game/Blueprints/Enums/ItemsList` (`self.Item`)
    (:`NewEnumerator2`
      (`/Game/Placeable/Player.GiveAmmo` (`self.Player`) (`self.GiveAmmo`)))
    (:`NewEnumerator3`
      (`/Game/Placeable/Player.GiveAmmo` (`self.Player`) (`self.GiveAmmo`)))
    (:`NewEnumerator18`
      (`KismetArrayLibrary.Array_AddUnique` (`/Game/Placeable/Player.MusketPartsStorage` (`self.Player`)) "Butt"))
    (:`NewEnumerator19`
      (`KismetArrayLibrary.Array_AddUnique` (`/Game/Placeable/Player.MusketPartsStorage` (`self.Player`)) "Body"))
    (:`NewEnumerator20`
      (`KismetArrayLibrary.Array_AddUnique` (`/Game/Placeable/Player.MusketPartsStorage` (`self.Player`)) "Trigger"))
    (:`NewEnumerator21`
      (`KismetArrayLibrary.Array_AddUnique` (`/Game/Placeable/Player.MusketPartsStorage` (`self.Player`)) "Pipe"))
    (:`NewEnumerator22`
      (`KismetArrayLibrary.Array_AddUnique` (`/Game/Placeable/Player.MusketPartsStorage` (`self.Player`)) "IronSight"))))

(fn `RotateMesh`
  (`SceneComponent.K2_SetRelativeLocationAndRotation` (`self.StaticMesh`) (`self.MeshLocation`) (`self.ItemRotation`) false false))

(fn `SetBoxSize`
  (bind _box (`self.Box`))
  (`BoxComponent.SetBoxExtent` _box (`self.TriggerBoxSize`) true)
  (`SceneComponent.K2_SetRelativeLocation` _box (`self.BoxLocation`) false false))

(fn `SetSettings`
  (params (Item :type "/Game/Blueprints/Enums/ItemsList Enum" :default "NewEnumerator17"))
  (bind _output_get (set `self.Item` Item))
  (bind _returnvalue (`|GetDataTableRow` "/Game/Blueprints/Enums/ItemData.ItemData" (`KismetStringLibrary.Conv_StringToName` (`KismetStringLibrary.Conv_ByteToString` _output_get)))
    (:`then`
      (bind (_item _info _mesh _particle) (break `/Game/Blueprints/Enums/ItemInfo` _returnvalue))
      (`StaticMeshComponent.SetStaticMesh` (`self.StaticMesh`) _mesh)
      (`ParticleSystemComponent.SetTemplate` (`self.P_Particle`) _particle)
      (set `self.ItemName` (`KismetTextLibrary.Conv_StringToText` (`|GetEnumeratorNameAsString` _item))))))

(fn `SetWidgetVisibility`
  (params (Visibility :type "ESlateVisibility Enum" :default "Visible"))
  (bind _itemname (`/Game/Blueprints/Widgets/Prototype_Item_Pickup.ItemName` (`self.HUD`)))
  (`Widget.SetVisibility` _itemname Visibility)
  (`Widget.SetVisibility` (`/Game/Blueprints/Widgets/Prototype_Item_Pickup.KeyToPress` (`self.HUD`)) Visibility)
  (`TextBlock.SetText` _itemname (`self.ItemName`)))

(fn `UserConstructionScript`
  (`self.SetBoxSize`)
  (`self.SetSettings` (`self.Item`))
  (`self.RotateMesh`))