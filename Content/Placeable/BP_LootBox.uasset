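; Placeable loot box that gives the player one preset item: a regular or superior first aid kit or ammo.
; Box overlap shows a pickup widget, reading "Locked" when locked, otherwise showing the data-table name and enabling interact input.
; Interacting once plays timelines that swing the lid open and raise the timer-spun item mesh.
; GiveItem then updates the player's inventory, and the mesh hides after a short delay.
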(event `self.ReceiveBeginPlay`
  (bind _returnvalue (`|CreateWidget` "/Game/Blueprints/Widgets/Prototype_Item_Pickup.Prototype_Item_Pickup_C"))
  (set `self.ItemPickUpHUD` _returnvalue)
  (`self.SetSettings`)
  (`self.SetItem`)
  (bind _asplayer (cast `/Game/Placeable/Player` (`GameplayStatics.GetPlayerCharacter` 0)))
  (set `self.Player` _asplayer))

(event `InputAction|Interact`
  (params (Key :type "Key Structure"))
  (bind _staticmesh (`self.StaticMesh`))
  (:`Pressed`
    (`StaticMeshComponent.SetStaticMesh` (`self.Lock`) null)
    (if (not (`/Game/Placeable/Player.bIsDead` (`self.Player`)))
      (`/Engine/EditorBlueprintResources/StandardMacros.DoOnce` false
        (:`Completed`
          (`Widget.RemoveFromParent` (`self.ItemPickUpHUD`))
          (`self.DisableInput` (`GameplayStatics.GetPlayerController` 0))
          (bind (_direction _y_axis) (`Timeline|Open`)
            (:`Update`
              (`SceneComponent.K2_SetRelativeRotation` (`self.CoverOrigin`) (`KismetMathLibrary.MakeRotator` 0.0 _y_axis) false false))
            (:`Finished`
              (`KismetSystemLibrary.K2_SetTimer` null "RotateItem" 0.01 true)
              (`SceneComponent.SetHiddenInGame` _staticmesh false false)
              (`SceneComponent.SetRelativeScale3D` _staticmesh (0.35 0.35 0.35))
              (set `self.IsLocked` false)
              (bind (_direction_2 _y_axis_2) (`Timeline|ShowItem` :!via `PlayFromStart`)
                (:`Update`
                  (`SceneComponent.K2_SetRelativeLocation` (`self.StaticMesh`) (`KismetMathLibrary.MakeVector` 0.0 0.0 _y_axis_2) false false))
                (:`Finished`
                  (`TextRenderComponent.K2_SetText` (`self.TextRender`) (`self.SelectedItemName`))
                  (`self.GiveItem`)
                  (`KismetSystemLibrary.Delay` 4.0)
                  (`SceneComponent.SetHiddenInGame` (`self.StaticMesh`) true false)
                  (`TextRenderComponent.K2_SetText` (`self.TextRender`) (`self.EmptyName`)))))))))))

(event `self.Box.OnComponentBeginOverlap`
  (params (OverlappedComponent :type "PrimitiveComponent Object Reference") (OtherActor :type "Actor Object Reference") (OtherComp :type "PrimitiveComponent Object Reference") (OtherBodyIndex :type Integer) (bFromSweep :type Boolean) (SweepResult :type "HitResult Structure (by ref)"))
  (cast `/Game/Placeable/Player` OtherActor)
  (if (`/Game/Placeable/Player.bIsDead` (`self.Player`))
    _
    (elif (`self.IsLocked`)
      (`self.WidgetWork` :!label _label)
      (elif (not (`self.bIsOverlapping`))
        (goto _label)))))

(event `self.Box.OnComponentEndOverlap`
  (params (OverlappedComponent :type "PrimitiveComponent Object Reference") (OtherActor :type "Actor Object Reference") (OtherComp :type "PrimitiveComponent Object Reference") (OtherBodyIndex :type Integer))
  (cast `/Game/Placeable/Player` OtherActor)
  (if (`/Game/Placeable/Player.bIsDead` (`self.Player`))
    _
    (elif (`self.IsLocked`)
      (goto _label :!via `Off`)
      (elif (`self.bIsOverlapping`)
        (goto _label :!via `Off`)))))

(event `RotateItem`
  (`SceneComponent.K2_AddLocalRotation` (`self.StaticMesh`) (struct :`Yaw` 1.0) false false))

(fn `GiveItem`
  (bind _player (`self.Player`))
  (bind _player_2 (`self.Player`))
  (bind _player_3 (`self.Player`))
  (switch `/Game/Blueprints/Enums/ItemsList` (`self.Item`)
    (:`NewEnumerator0`
      (`KismetArrayLibrary.Array_Add` (`/Game/Placeable/Player.Collection` _player_3) "FirstAidKit")
      (set `/Game/Placeable/Player.FirstAidKitCount` (+ (`/Game/Placeable/Player.FirstAidKitCount` _player_3) 1) _player_3))
    (:`NewEnumerator1`
      (`KismetArrayLibrary.Array_Add` (`/Game/Placeable/Player.Collection` _player) "SuperiorFirstAidKit")
      (set `/Game/Placeable/Player.SuperiorFirstAidKitCount` (+ (`/Game/Placeable/Player.SuperiorFirstAidKitCount` _player) 1) _player))
    (:`NewEnumerator2`
      (`/Game/Placeable/Player.GiveAmmo` (`self.Player`) 1)
      (`KismetArrayLibrary.Array_Add` (`/Game/Placeable/Player.Collection` _player_2) "Ammo")
      (set `/Game/Placeable/Player.AmmoCount` (+ (`/Game/Placeable/Player.AmmoCount` _player_2) 1) _player_2))
    (:`NewEnumerator3`
      (`/Game/Placeable/Player.GiveAmmo` (`self.Player`) 3)
      (`KismetArrayLibrary.Array_Add` (`/Game/Placeable/Player.Collection` (`self.Player`)) "SuperiorAmmo"))))

(fn `SetItem`
  (switch `/Game/Blueprints/Enums/ItemsList` (`self.Item`)
    (:`NewEnumerator0`
      (`StaticMeshComponent.SetStaticMesh` (`self.StaticMesh`) "/Game/Meshes/MESH_FirstAidKit.MESH_FirstAidKit")
      (set `self.SelectedItemName` "First Aid Kit"))
    (:`NewEnumerator1`
      (`StaticMeshComponent.SetStaticMesh` (`self.StaticMesh`) "/Game/Meshes/MESH_SuperiorFirstAidKit.MESH_SuperiorFirstAidKit")
      (set `self.SelectedItemName` "Superior First Aid Kit"))
    (:`NewEnumerator2`
      (`StaticMeshComponent.SetStaticMesh` (`self.StaticMesh`) "/Game/Meshes/MESH_Ammo.MESH_Ammo")
      (set `self.SelectedItemName` "Ammo"))
    (:`NewEnumerator3`
      (`StaticMeshComponent.SetStaticMesh` (`self.StaticMesh`) "/Game/Meshes/MESH_SuperiorAmmo.MESH_SuperiorAmmo")
      (set `self.SelectedItemName` "Supeior Ammo"))))

(fn `SetSettings`
  (bind _returnvalue (`|GetDataTableRow` "/Game/Blueprints/Enums/ItemData.ItemData" "20")
    (:`then`
      (set `self.SelfName` (`KismetTextLibrary.Conv_StringToText` (`|GetEnumeratorNameAsString` (`.Item_40_4AC5B1F34F15103FA5B55388B1388A81` (break `/Game/Blueprints/Enums/ItemInfo` _returnvalue))))))))

(fn `SetWidgetVisibility`
  (params (InVisibility :type "ESlateVisibility Enum" :default "Visible"))
  (bind _itemname (`/Game/Blueprints/Widgets/Prototype_Item_Pickup.ItemName` (`self.ItemPickUpHUD`)))
  (`Widget.SetVisibility` _itemname InVisibility)
  (`Widget.SetVisibility` (`/Game/Blueprints/Widgets/Prototype_Item_Pickup.KeyToPress` (`self.ItemPickUpHUD`)) InVisibility)
  (`TextBlock.SetText` _itemname (`self.SelfName`)))

(fn `UserConstructionScript`)